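; Showcase Blueprint for the West M983 HEMTT truck that exposes its adjustable parts to generic showcase controls.
; Indexed slider, twin slider, checkbox and button events forward their values to setters for doors, mirrors, window cleaners, wheel speed and angle, light emissivity, damage display and skin type.
; It holds only this control mapping, and its construction script just calls the parent's.
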(event EventSetSliderVariable2
  (params (NewValue :type Float%20%28single-precision%29))
  ;[1 1 1] Showcase float controls
  (CallFunction|SetLightsEmissivity NewValue))

(event EventSetSliderVariable1
  (params (NewValue :type Float%20%28single-precision%29))
  ;[1 1 1] Showcase float controls
  (CallFunction|SetWheelAngle NewValue))

(event EventSetCheckboxVariable0
  (params (NewState :type Boolean))
  ;[1 1 1] Showcase checkbox controls
  (CallFunction|SetShowDamaged NewState))

(event EventSetButtonsVariable0
  (params (NewIndex :type Integer))
  ;[1 1 1] Showcase button controls
  (CallFunction|SetSkinType (Math|Conversions|ToFloat(Integer) NewIndex)))

(event EventSetTwinSliderVariable0
  (params (bFirstSlider? :type Boolean) (NewFirstValue :type Float%20%28single-precision%29) (NewSecondValue :type Float%20%28single-precision%29))
  ;[1 1 1] Showcase twin float controls
  (CallFunction|SetDoors NewFirstValue NewSecondValue))

(event EventSetTwinSliderVariable1
  (params (bFirstSlider? :type Boolean) (NewFirstValue :type Float%20%28single-precision%29) (NewSecondValue :type Float%20%28single-precision%29))
  ;[1 1 1] Showcase twin float controls
  (CallFunction|SetMirrors NewFirstValue NewSecondValue))

(event EventSetTwinSliderVariable2
  (params (bFirstSlider? :type Boolean) (NewFirstValue :type Float%20%28single-precision%29) (NewSecondValue :type Float%20%28single-precision%29))
  ;[1 1 1] Showcase twin float controls
  (CallFunction|SetWindowCleaners NewFirstValue NewSecondValue))

(event EventSetSliderVariable0
  (params (NewValue :type Float%20%28single-precision%29))
  ;[1 1 1] Showcase float controls
  (CallFunction|SetWheelSpeed NewValue))

(fn ConstructionScript
  (|CallParentFunction))