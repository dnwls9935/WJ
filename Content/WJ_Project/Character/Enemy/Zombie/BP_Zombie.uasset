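; BP_Zombie is a zombie enemy Character with location-based damage and destructible legs.
; Hit passes the hit bone name to ShootTarget, which doubles head damage and halves leg damage, then CalcurationDamage subtracts the result from CurrentHealth.
; Each leg tracks its own health and halves movement speed once when depleted.
; Die ragdolls the mesh and removes the capsule but is not called here, and the health bar update is disconnected.
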(event EventBeginPlay)

(fn ConstructionScript
  (|CallParentFunction))

(fn Hit
  (params (name :type String) (damage :type Float%20%28double-precision%29))
  (CallFunction|ShootTarget name damage)
  (디폴트|CalcurationDamage))

(fn CalcurationDamage
  (Variables|Default|Setcurrent_health (- (Variables|Default|Getcurrent_health) (Variables|Default|GetCal%20Damage)))
  (Variables|Default|SetCal%20Damage 0.0))

(fn RightLegShoot
  (params (Cal%20Damage :type Float%20%28double-precision%29) (B :type Float%20%28double-precision%29)))

(fn ShootTarget
  (params (Selection :type String) (Damage :type Float%20%28double-precision%29))
  (bind _returnvalue (/ Damage 2.0))
  (bind _charactermovement (Variables|Character|GetCharacterMovement))
  (switch string Selection
    (:head
      (Variables|Default|SetCal%20Damage (* Damage 2.0)))
    (:spine_0
      (Variables|Default|SetCal%20Damage Damage))
    (:calf_l
      (bind _output_get (Variables|Default|Setleft_leg_health (- (Variables|Default|Getleft_leg_health) Damage) :!label _label))
      (if (and (<= _output_get 0.0) (== (Variables|Default|Getleft_leg_destroy) false))
        (Variables|Default|Setleft_leg_health 0.0)
        (Variables|Default|Setleft_leg_destroy true)
        (bind _output_get_2 (Variables|/Script/Engine.CharacterMovementComponent|SetMaxWalkSpeed _charactermovement (/ (Variables|Default|Getmovement_speed) 2.0)))
        (Variables|Default|Setmovement_speed _output_get_2))
      (Variables|Default|SetCal%20Damage _returnvalue))
    (:foot_l
      (goto _label))
    (:claf_r
      (bind _output_get_3 (Variables|Default|Setright_leg_health (- (Variables|Default|Getright_leg_health) Damage) :!label _label_2))
      (if (and (== (Variables|Default|Getright_leg_destroy) false) (<= _output_get_3 0.0))
        (Variables|Default|Setright_leg_health 0.0)
        (Variables|Default|Setright_leg_destroy true)
        (bind _output_get_4 (Variables|/Script/Engine.CharacterMovementComponent|SetMaxWalkSpeed _charactermovement (/ (Variables|Default|Getmovement_speed) 2.0)))
        (Variables|Default|Setmovement_speed _output_get_4))
      (Variables|Default|SetCal%20Damage _returnvalue))
    (:foot_r
      (goto _label_2))))

(fn Die
  (bind _capsulecomponent (Variables|Default|GetCapsuleComponent))
  (Physics|SetSimulatePhysics (Variables|Character|GetMesh) true)
  (Utilities|IsValid _capsulecomponent
    (:Is%20Valid
      (Components|DestroyComponent _capsulecomponent))))