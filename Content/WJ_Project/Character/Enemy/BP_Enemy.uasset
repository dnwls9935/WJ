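; Enemy character that tracks health from point damage and handles its own death.
; Each point damage event calls Die when the damage would deplete health, otherwise Hit with the struck component's name, then subtracts the damage.
; Die sets a one-time dead flag and destroys the actor after a timed delay, while Hit only passes its inputs back out.
; The construction script copies the movement component's max custom movement speed into MovementSpeed.
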(event Game|Damage|EventPointDamage
  (params (Damage :type Float%20%28single-precision%29) (DamageType :type Damage%20Type%20Object%20Reference) (HitLocation :type Vector :default "0, 0, 0") (HitNormal :type Vector :default "0, 0, 0") (HitComponent :type Primitive%20Component%20Object%20Reference) (BoneName :type Name :default "None") (ShotFromDirection :type Vector :default "0, 0, 0") (InstigatedBy :type Controller%20Object%20Reference) (DamageCauser :type Actor%20Object%20Reference) (HitInfo :type Hit%20Result%20Structure%20%28by%20ref%29))
  (if (<= (- (Variables|Default|Getcurrent_health) Damage) 0.0)
    (CallFunction|Die)
    (else
      (디폴트|Hit (Utilities|GetObjectName HitComponent) Damage)))
  (Variables|Default|Setcurrent_health (- (Variables|Default|Getcurrent_health) Damage)))

(fn ConstructionScript
  (Variables|Default|SetMovement%20Speed (Variables|/Script/Engine.CharacterMovementComponent|GetMaxCustomMovementSpeed (Variables|Character|GetCharacterMovement))))

(fn Hit
  (params (name :type String) (damage :type Float%20%28double-precision%29))
  (return name damage))

(fn Die
  (if (not (Variables|Default|Getis_dead))
    (Variables|Default|Setis_dead true)
    (Utilities|Time|SetTimerbyFunctionName self "Destroy" 1e+01)))

(fn Destroy
  (Actor|DestroyActor))